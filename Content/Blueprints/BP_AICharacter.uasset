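; BP_AICharacter is an AI character that chases the player when it is allowed to attack.
; BeginPlay casts player character 0 to BP_PlayerCharacter and caches the reference.
; While CanAttack is true, every Tick calls GoToPlayer, which reissues AI MoveTo with that cached player as the target actor.
; The graph contains no attack logic and never sets CanAttack itself.
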(event `self.ReceiveBeginPlay`
  (bind _asbp_player_character (cast `/Game/Blueprints/BP_PlayerCharacter` (`GameplayStatics.GetPlayerCharacter` 0)))
  (set `self.As BP Player Character` _asbp_player_character))

(event `self.ReceiveTick`
  (params (DeltaSeconds :type "Float (single-precision)"))
  (if (`self.bCanAttack`)
    (`self.GoToPlayer`)))

(event `GoToPlayer`
  (`|AIMoveTo` self (`self.K2_GetActorLocation`) (`self.As BP Player Character`)))

(fn `UserConstructionScript`)